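; BP_TestSave is a test Blueprint for the save system, working with a BP_Save object in the GameSave slot.
; On BeginPlay it loads and caches the existing save, or creates, writes and caches a new one.
; Unconnected fragments sketch two save variants and a load step that sets the player controller's transform without reading saved data; none of them run.
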(event `self.ReceiveBeginPlay`
  (bind _returnvalue (`GameplayStatics.DoesSaveGameExist` "GameSave"))
  (if _returnvalue
    (bind _returnvalue_2 (`GameplayStatics.LoadGameFromSlot` "GameSave"))
    (bind _asbp_save (cast `/Game/Menus/SaveSystem/BP_Save` _returnvalue_2))
    (set `self.As BP Save` _asbp_save)
    (else
      (bind _returnvalue_3 (`GameplayStatics.CreateSaveGameObject` "/Game/Menus/SaveSystem/BP_Save.BP_Save_C"))
      (`GameplayStatics.SaveGameToSlot` _returnvalue_3 "GameSave")
      (set `self.As BP Save` _returnvalue_3))))

(fn `UserConstructionScript`)